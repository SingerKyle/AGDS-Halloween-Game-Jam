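; BP_Pipe is a smokable pipe prop that can be placed on a pumpkin character.
; On grip release, a small sphere trace at its Scene component searches a single object type.
; A hit on a BP_PumpkinCharacter snaps the pipe to that character's PipeAttachment, keeping world scale.
; With no hit, it detaches and teleports back to its stored initial location and rotation.
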(event EventBeginPlay
  (|CallParentFunction) ; This node is disabled and will not be called.\nDrag off pins to build functionality.
)

(event Collision|EventActorBeginOverlap
  (params (OtherActor :type Actor%20Object%20Reference))
  (|CallParentFunction OtherActor) ; This node is disabled and will not be called.\nDrag off pins to build functionality.
)

(event EventTick
  (params (DeltaSeconds :type Float%20%28single-precision%29))
  (|CallParentFunction DeltaSeconds) ; This node is disabled and will not be called.\nDrag off pins to build functionality.
)

(event EventOnGripRelease
  (params (ReleasingController :type Grip%20Motion%20Controller%20Component%20Object%20Reference) (GripInformation :type BP%20Actor%20Grip%20Information%20Structure%20%28by%20ref%29) (bWasSocketed :type Boolean))
  (bind _scene (Variables|Default|GetScene))
  (bind _returnvalue (Transformation|GetWorldLocation _scene))
  (bind (_outhit _returnvalue_2) (Collision|SphereTraceForObjects _returnvalue _returnvalue 12.0 (Utilities|Array|MakeArray "ObjectTypeQuery7") false 0 "None"))
  (if _returnvalue_2
    (bind _asbp_pumpkin_character (Utilities|Casting|CastToBP_PumpkinCharacter (.HitActor (Collision|BreakHitResult _outhit))))
    (Transformation|AttachComponentToComponent (Variables|/Game/PumpkinRoulette/Blueprint/BP_PumpkinCharacter.BP_PumpkinCharacter_C|GetPipeAttachment _asbp_pumpkin_character) "None" "SnapToTarget" "SnapToTarget" "KeepWorld" false)
    (else
      (Transformation|DetachFromActor "KeepRelative" "KeepRelative" "KeepRelative")
      (Transformation|SetActorLocationAndRotation (Variables|Default|GetInitialLocation) (Variables|Default|GetInitialRotation) false true))))

(fn ConstructionScript
  (|CallParentFunction))